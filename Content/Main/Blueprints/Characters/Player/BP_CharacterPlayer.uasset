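; BP_CharacterPlayer is the player character Blueprint, with a hold-right-mouse stance that appears to be an aim mode.
; Pressing moves the camera to a fixed offset, swaps the animation class to ABP_Character and makes the body follow controller rotation.
; Releasing restores the camera transform cached at BeginPlay, ABP_Manny and movement-oriented rotation, but leaves controller yaw and roll enabled.
; The F key plays a test camera shake with a debug print.
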(event EventBeginPlay
  (Variables|Default|SetCameraInitialTransform (Transformation|GetRelativeTransform (Variables|Default|GetCameraComponent))))

(event Input|MouseEvents|RightMouseButton
  (params (Key :type Key%20Structure :default "None"))
  (bind _mesh (Variables|Character|GetMesh))
  (bind _camerainitialtransform (Variables|Default|GetCameraInitialTransform))
  (bind _mesh_2 (Variables|Character|GetMesh))
  (bind (_location _rotation) (Math|Transform|BreakTransform _camerainitialtransform))
  (:Pressed
    (Components|MoveComponentTo (Variables|Default|GetCameraComponent) "300.000000,50.000000,25.000000" "0, 0, 0" false false 0.2 false)
    (Components|Animation|SetAnimationMode _mesh "AnimationBlueprint")
    (Class|SkeletalMeshComponent|SetAnimClass _mesh "/Game/Main/Blueprints/Characters/ABP_Character.ABP_Character_C")
    (Variables|/Script/Engine.CharacterMovementComponent|SetbOrientRotationToMovement (Variables|Character|GetCharacterMovement) false)
    (Variables|/Script/Engine.CameraComponent|SetbUsePawnControlRotation (Variables|Default|GetCameraComponent) false)
    (Variables|Default|SetbUseControllerRotationYaw true)
    (Variables|Default|SetbUseControllerRotationRoll true))
  (:Released
    (Components|MoveComponentTo (Variables|Default|GetCameraComponent) _location _rotation false false 0.2 false)
    (Components|Animation|SetAnimationMode _mesh_2 "AnimationBlueprint")
    (Class|SkeletalMeshComponent|SetAnimClass _mesh_2 "/Game/Characters/Mannequins/Animations/ABP_Manny.ABP_Manny_C")
    (Variables|/Script/Engine.CharacterMovementComponent|SetbOrientRotationToMovement (Variables|Character|GetCharacterMovement) true)
    (Variables|/Script/Engine.CameraComponent|SetbUsePawnControlRotation (Variables|Default|GetCameraComponent) false)))

(event Input|KeyboardEvents|F
  (params (Key :type Key%20Structure :default "None"))
  (:Pressed
    (Camera|PlayWorldCameraShake "/Game/Main/Blueprints/Characters/Camera/BP_CameraShake.BP_CameraShake_C" (Transformation|GetWorldLocation (Variables|Default|GetCameraComponent)) 15.0 15.0 15.0)
    (Development|PrintString "Hello")))

(fn ConstructionScript)