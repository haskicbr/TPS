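; Player character Blueprint that handles camera repositioning and a test camera shake.
; BeginPlay caches the camera's relative transform, which releasing the right mouse button restores through MoveComponentTo.
; Holding that button moves the camera to a fixed relative offset.
; The F key plays a world camera shake centered on the camera and prints a debug string.
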(event EventBeginPlay
  (Variables|Default|SetCameraInitialTransform (Transformation|GetRelativeTransform (Variables|Default|GetCameraComponent))))

(event Input|MouseEvents|RightMouseButton
  (params (Key :type Key%20Structure :default "None"))
  (bind _camerainitialtransform (Variables|Default|GetCameraInitialTransform))
  (bind (_location _rotation) (Math|Transform|BreakTransform _camerainitialtransform))
  (:Pressed
    (Components|MoveComponentTo (Variables|Default|GetCameraComponent) "-25.000000,0.000000,50.000000" "0, 0, 0" false false 0.2 false))
  (:Released
    (Components|MoveComponentTo (Variables|Default|GetCameraComponent) _location _rotation false false 0.2 false)))

(event Input|KeyboardEvents|F
  (params (Key :type Key%20Structure :default "None"))
  (:Pressed
    (Camera|PlayWorldCameraShake "/Game/Main/Blueprints/Characters/Camera/BP_CameraShake.BP_CameraShake_C" (Transformation|GetWorldLocation (Variables|Default|GetCameraComponent)) 15.0 15.0 15.0)
    (Development|PrintString "Hello")))

(fn ConstructionScript)