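; Trailer vehicle Blueprint that hitches itself to a referenced Truck when play begins.
; If the Truck is valid and casts to WheelPawn, it sets a small throttle input on both the truck's and its own Chaos vehicle movement components.
; A physics constraint then joins the trailer mesh to the truck mesh.
; An alternative cast to OffroadCar_Pawn is left unconnected and never runs.
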(event EventBeginPlay
  (bind _truck (Variables|Default|GetTruck))
  (Utilities|IsValid _truck
    (:Is%20Valid
      (bind _aswheel_pawn (Utilities|Casting|CastToWheelPawn _truck))
      (Class|ChaosVehicleMovementComponent|SetThrottleInput (Actor|GetComponentbyClass _truck "/Script/ChaosVehicles.ChaosWheeledVehicleMovementComponent") 0.1)
      (Class|PhysicsConstraintComponent|SetConstrainedComponents (Variables|Default|GetPhysicsConstraint) (Variables|Character|GetMesh) "None" (Variables|/Script/ChaosVehicles.WheeledVehiclePawn|GetMesh _aswheel_pawn) "None"))))

(fn ConstructionScript)