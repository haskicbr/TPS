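; BP_Slice is a test actor that cuts its Cube mesh with a plane when play begins.
; On BeginPlay it copies the Cube static mesh into a ProceduralMesh component, then slices that copy through the actor's location along the cube's forward vector.
; The cut is capped using the last mesh section, and the original Cube component is destroyed, leaving the procedural result.
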(event EventBeginPlay
  (Class|KismetProceduralMeshLibrary|CopyProceduralMeshfromStaticMeshComponent (Variables|Default|GetCube) 0 (Variables|Default|GetProceduralMesh) false)
  (Class|KismetProceduralMeshLibrary|SliceProceduralMesh (Variables|Default|GetProceduralMesh) (Transformation|GetActorLocation) (* (Math|Vector|GetForwardVector (Variables|Default|GetCube)) 111) false "UseLastSectionForCap" "/Engine/MaterialTemplates/VertexAnimation/AdvancedFlag.AdvancedFlag")
  (Components|DestroyComponent (Variables|Default|GetCube)))

(event Collision|EventActorBeginOverlap
  (params (OtherActor :type Actor%20Object%20Reference)))

(event EventTick
  (params (DeltaSeconds :type Float%20%28single-precision%29)))

(fn ConstructionScript)